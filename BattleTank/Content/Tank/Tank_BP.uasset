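; Player-controllable tank Blueprint, built on the C++ Tank class, that binds input to aiming, movement, camera and firing.
; On BeginPlay it passes the barrel and turret to TankAiming and both tracks to TankMovement.
; Move and turn axes feed TankMovement intents, while Fire calls the C++ method.
; Camera yaw rotates AzimuthGimbal and pitch rotates SpringArm separately to avoid unwanted rotation, both scaled by delta time.
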(event EventBeginPlay
  (Class|TankAimingComponent|Initialise (Variables|Default|GetTankAiming) (Variables|Default|GetBarrel) (Variables|Default|GetTurret))
  (Class|TankMovementComponent|Initialise (Variables|Default|GetTankMovement) (Variables|Default|GetLeftTrack) (Variables|Default|GetRightTrack)))

(event Input|ActionEvents|InputActionFire
  (params (Key :type Key%20Structure :default "AnyKey"))
  ;[1 1 1] This controls the the yaw and pitch of the camera, making sure that when we move the pitch and yaw together it doesnt rotate
  (:Pressed
    ;;[1 1 1] Method from the c++ class Tank
    (Class|Tank|Fire)))

(event Input|AxisEvents|InputAxisMoveForward
  (params (AxisValue :type Float%20%28single-precision%29))
  ;[1 1 1] Throttle input
  (Class|TankMovementComponent|IntendMoveForward (Variables|Default|GetTankMovement) AxisValue))

(event Input|AxisEvents|InputAxisTurnRight
  (params (AxisValue :type Float%20%28single-precision%29))
  ;[1 1 1] Throttle input
  (Class|TankMovementComponent|IntendTurnRight (Variables|Default|GetTankMovement) AxisValue))

(event Input|AxisEvents|InputAxisAimAzimuth
  (params (AxisValue :type Float%20%28single-precision%29))
  ;[1 1 1] This controls the the yaw and pitch of the camera, making sure that when we move the pitch and yaw together it doesnt rotate
  (Transformation|AddLocalRotation (Variables|Default|GetAzimuth%20Gimbal) (Math|Rotator|MakeRotator 0.0 0.0 (* AxisValue (Utilities|Time|GetWorldDeltaSeconds) 1e+02)) false false))

(event Input|AxisEvents|InputAxisAimElevation
  (params (AxisValue :type Float%20%28single-precision%29))
  ;[1 1 1] This controls the the yaw and pitch of the camera, making sure that when we move the pitch and yaw together it doesnt rotate
  (Transformation|AddLocalRotation (Variables|Default|GetSpringArm) (Math|Rotator|MakeRotator 0.0 (* AxisValue (Utilities|Time|GetWorldDeltaSeconds) 1e+02) 0.0) false false))

(fn ConstructionScript)